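; BP_Athel is the player character, a directional 2D sprite character handling movement, sword attacks, NPC talk, HUD and journal menus.
; Movement input feeds sprite directionality, which rotates a front-facing collision box and steers attack pushes from a timeline.
; Attacks send combo requests to the animation instance, while menu keys play a book animation and record which journal page to open.
; Debug keys test multi-slot saving and health.
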(event OnComponentBeginOverlap(BoxCollision)
  (params (OverlappedComponent :type Primitive%20Component%20Object%20Reference) (OtherActor :type Actor%20Object%20Reference) (OtherComp :type Primitive%20Component%20Object%20Reference) (OtherBodyIndex :type Integer) (bFromSweep :type Boolean) (SweepResult :type Hit%20Result%20Structure%20%28by%20ref%29))
  ;[1 1 1] BeginOverlap of BoxCollision to check if overlapping actor is NPC and has PromptCollision tag on a component. If yes, sets InteractBox to on. When it leaves, turns off.
  (CallFunction|IfOverlappingNPC OtherActor OtherComp))

(event OnComponentEndOverlap(BoxCollision)
  (params (OverlappedComponent :type Primitive%20Component%20Object%20Reference) (OtherActor :type Actor%20Object%20Reference) (OtherComp :type Primitive%20Component%20Object%20Reference) (OtherBodyIndex :type Integer))
  ;[1 1 1] BeginOverlap of BoxCollision to check if overlapping actor is NPC and has PromptCollision tag on a component. If yes, sets InteractBox to on. When it leaves, turns off.
  (CallFunction|NPCLeavesOverlap OtherActor OtherComp))

(event Custom|AttackMovement_Update
  ;[1 1 1] Controls forward movement during attack animation
  (bind (_direction _x _y) (Timeline|MovingAttack PlayFromStart)
    (:Update
      (CallFunction|PushMoveForward _x _y))))

(event Custom|Open%20Menu
  (bind _currentkey (Variables|Default|GetCurrentKey))
  ;[1 1 1] Open Menu
  (CallFunction|OpenPlayerMenu _currentkey)
  (if (== _currentkey "I")
    (Default|DEBUGPrintContents (Variables|Default|GetInventory))))

(event EventBeginPlay
  ;[1 1 1] INIT ON PLAY
  (Utilities|FlowControl|Sequence
    (:then_0
      (CallFunction|CreateHUD)
      (bind _astcm_game_instance (Utilities|Casting|CastToTCM_GameInstance (Game|GetGameInstance)))
      (Variables|Default|SetTCM%20Game%20Instance _astcm_game_instance))))

(event EventTick
  (params (DeltaSeconds :type Float%20%28single-precision%29))
  ;[1 1 1] Rotates BoxHolder to orient BoxCollision around the player. (exists to check what's infront of player)
  (CallFunction|SetBoxRotationAroundPlayer)
  (bind _astcm_game_instance (Utilities|Casting|CastToTCM_GameInstance (Game|GetGameInstance))))

(event Input|AxisEvents|InputAxisMoveRight
  (params (AxisValue :type Float%20%28single-precision%29))
  ;[1 1 1] Controls Character Movement and passes IsHoldingMove = true while running.
  (if (not (Variables|Default|GetIsMovementLocked))
    (Variables|Default|SetIsHoldingMove true)
    (Pawn|Input|AddMovementInput (Math|Vector|GetRightVector (Pawn|GetControlRotation :!class /Script/Engine.Pawn)) AxisValue false)
    ;[1 1 1] Checks If Character is moving in any direction before passing to Set IsHoldingMove = false
    (if (== AxisValue 0.0)
      (if (== (stale Input|AxisEvents|InputAxisMoveUp AxisValue) 0.0)
        (Variables|Default|SetIsHoldingMove false)
        (else
          (Variables|/Game/BluePrints/Components/Paper2DActor.Paper2DActor_C|SetDirectionality (Variables|Default|GetPaper2DActor) (Math|Vector2D|MakeVector2D AxisValue (stale Input|AxisEvents|InputAxisMoveUp AxisValue)) :!label _label)))
      (else
        (goto _label)))))

(event Input|AxisEvents|InputAxisMoveUp
  (params (AxisValue :type Float%20%28single-precision%29))
  ;[1 1 1] Controls Character Movement and passes IsHoldingMove = true while running.
  (if (not (Variables|Default|GetIsMovementLocked))
    (Variables|Default|SetIsHoldingMove true)
    (Pawn|Input|AddMovementInput (Math|Vector|GetForwardVector (Pawn|GetControlRotation :!class /Script/Engine.Pawn)) AxisValue false)
    ;[1 1 1] Checks If Character is moving in any direction before passing to Set IsHoldingMove = false
    (if (== (stale Input|AxisEvents|InputAxisMoveRight AxisValue) 0.0)
      (if (== AxisValue 0.0)
        (Variables|Default|SetIsHoldingMove false)
        (else
          (Variables|/Game/BluePrints/Components/Paper2DActor.Paper2DActor_C|SetDirectionality (Variables|Default|GetPaper2DActor) (Math|Vector2D|MakeVector2D (stale Input|AxisEvents|InputAxisMoveRight AxisValue) AxisValue) :!label _label)))
      (else
        (goto _label)))))

(event Input|KeyboardEvents|E
  (params (Key :type Key%20Structure :default "None"))
  (bind _self self)
  ;[1 1 1] Checks If NPC Actor is within range to talk after pressing E Key.
  (:Pressed
    (bind _returnvalue (CallFunction|NPCCheck))
    (Utilities|IsValid _self
      (:Is%20Valid
        (Default|Talk _returnvalue _self)))))

(event Input|GamepadEvents|GamepadFaceButtonLeft
  (params (Key :type Key%20Structure :default "None"))
  (bind _self self)
  ;[1 1 1] Checks If NPC Actor is within range to talk after pressing E Key.
  (:Pressed
    (bind _returnvalue (CallFunction|NPCCheck))
    (Utilities|IsValid _self
      (:Is%20Valid
        (Default|Talk _returnvalue _self)))))

(event Input|GamepadEvents|GamepadDPadUp
  (params (Key :type Key%20Structure :default "None"))
  ;[1 1 1] Open Menu
  ;;[1 1 1] Inventory
  (:Pressed
    (bind _canpass (CallFunction|PlayBookAnimation))
    (if _canpass
      (Variables|Default|SetCurrentKey "I"))))

(event Input|GamepadEvents|GamepadDPadRight
  (params (Key :type Key%20Structure :default "None"))
  ;[1 1 1] Open Menu
  ;;[1 1 1] Quests
  (:Pressed
    (bind _canpass (CallFunction|PlayBookAnimation))
    (if _canpass
      (Variables|Default|SetCurrentKey "L"))))

(event Input|GamepadEvents|GamepadDPadDown
  (params (Key :type Key%20Structure :default "None"))
  ;[1 1 1] Open Menu
  ;;[1 1 1] Index
  (:Pressed
    (bind _canpass (CallFunction|PlayBookAnimation))
    (if _canpass
      (Variables|Default|SetCurrentKey "J"))))

(event Input|GamepadEvents|GamepadDPadLeft
  (params (Key :type Key%20Structure :default "None"))
  ;[1 1 1] Open Menu
  ;;[1 1 1] Notes
  (:Pressed
    (bind _canpass (CallFunction|PlayBookAnimation))
    (if _canpass
      (Variables|Default|SetCurrentKey "K"))))

(event Input|KeyboardEvents|Left
  (params (Key :type Key%20Structure :default "None"))
  ;[1 1 1] Save/Load
  ;;[1 1 1] multi save slot test
  (:Pressed
    (Default|SavetoSlot (Variables|Default|GetTCM%20Game%20Instance) 0 "Title1")))

(event Input|KeyboardEvents|NumPadFive
  (params (Key :type Key%20Structure :default "None"))
  ;[1 1 1] Save/Load
  ;;[1 1 1] Save/Load Data test on CurrentHealth
  (:Pressed
    (bind _output_get (Variables|/Game/BluePrints/CombatSystems/BaseComponents/BPC_CMB_HealthComponent.BPC_CMB_HealthComponent_C|SetCurrentHealthPoints (Variables|Default|GetBPC_CMB_HealthComponent) 5e+01))
    (Development|PrintString (Utilities|String|ToString(Float) _output_get))))

(event Input|KeyboardEvents|Down
  (params (Key :type Key%20Structure :default "None"))
  ;[1 1 1] Save/Load
  ;;[1 1 1] multi save slot test
  (:Pressed
    (Default|SavetoSlot (Variables|Default|GetTCM%20Game%20Instance) 1 "Title2")))

(event Input|KeyboardEvents|J
  (params (Key :type Key%20Structure :default "None"))
  ;[1 1 1] Open Menu
  ;;[1 1 1] Index
  (:Pressed
    (bind _canpass (CallFunction|PlayBookAnimation))
    (if _canpass
      (Variables|Default|SetCurrentKey "J"))))

(event Input|KeyboardEvents|Right
  (params (Key :type Key%20Structure :default "None"))
  ;[1 1 1] Save/Load
  ;;[1 1 1] multi save slot test
  (:Pressed
    (Default|SavetoSlot (Variables|Default|GetTCM%20Game%20Instance) 2 "Title3")))

(event Input|KeyboardEvents|NumPadSeven
  (params (Key :type Key%20Structure :default "None"))
  (:Pressed
    (Default|DeleteSlot (Variables|Default|GetTCM%20Game%20Instance))))

(event Input|KeyboardEvents|LeftBracket
  (params (Key :type Key%20Structure :default "None"))
  ;[1 1 1] Save/Load
  ;;[1 1 1] multi save slot test
  (:Pressed
    (Default|LoadSlot (Variables|Default|GetTCM%20Game%20Instance) 1)))

(event Input|KeyboardEvents|RightBracket
  (params (Key :type Key%20Structure :default "None"))
  ;[1 1 1] Save/Load
  ;;[1 1 1] multi save slot test
  (:Pressed
    (Default|LoadSlot (Variables|Default|GetTCM%20Game%20Instance) 2)))

(event Input|KeyboardEvents|Up
  (params (Key :type Key%20Structure :default "None"))
  ;[1 1 1] Save/Load
  ;;[1 1 1] multi save slot test
  (:Pressed
    (Default|LoadSlot (Variables|Default|GetTCM%20Game%20Instance))))

(event Input|KeyboardEvents|NumPadEight
  (params (Key :type Key%20Structure :default "None"))
  (:Pressed
    (Default|DeleteSlot (Variables|Default|GetTCM%20Game%20Instance) 1)))

(event Input|KeyboardEvents|NumPadNine
  (params (Key :type Key%20Structure :default "None"))
  (:Pressed
    (Default|DeleteSlot (Variables|Default|GetTCM%20Game%20Instance) 2)))

(event Input|KeyboardEvents|I
  (params (Key :type Key%20Structure :default "None"))
  ;[1 1 1] Open Menu
  ;;[1 1 1] Inventory
  (:Pressed
    (bind _canpass (CallFunction|PlayBookAnimation))
    (if _canpass
      (Variables|Default|SetCurrentKey "I"))))

(event Input|MouseEvents|LeftMouseButton
  (params (Key :type Key%20Structure :default "None"))
  ;[1 1 1] Athel does attack. Checks Animation playing, then calls to attack component. Plays animation and stops player, then spawns particle effect.
  (:Pressed
    (if (Variables|Default|GetCanAttack)
      (Class|BPIComboRequest|RequestCombo(Message) (Variables|/Script/PaperZD.PaperZDAnimationComponent|GetAnimInstance (Variables|Default|GetAnimationComponent)) "NewEnumerator0"))))

(event Input|KeyboardEvents|Q
  (params (Key :type Key%20Structure :default "None"))
  ;[1 1 1] Open Menu
  ;;[1 1 1] Main Menu
  (:Pressed
    (CallFunction|PlayBookAnimation)))

(event Input|KeyboardEvents|L
  (params (Key :type Key%20Structure :default "None"))
  ;[1 1 1] Open Menu
  ;;[1 1 1] Quests
  (:Pressed
    (bind _canpass (CallFunction|PlayBookAnimation))
    (if _canpass
      (Variables|Default|SetCurrentKey "L"))))

(event Input|KeyboardEvents|K
  (params (Key :type Key%20Structure :default "None"))
  ;[1 1 1] Open Menu
  ;;[1 1 1] Notes
  (:Pressed
    (bind _canpass (CallFunction|PlayBookAnimation))
    (if _canpass
      (Variables|Default|SetCurrentKey "K"))))

(event Input|GamepadEvents|GamepadRightTrigger
  (params (Key :type Key%20Structure :default "None"))
  ;[1 1 1] Athel does attack. Checks Animation playing, then calls to attack component. Plays animation and stops player, then spawns particle effect.
  (:Pressed
    (if (Variables|Default|GetCanAttack)
      (Class|BPIComboRequest|RequestCombo(Message) (Variables|/Script/PaperZD.PaperZDAnimationComponent|GetAnimInstance (Variables|Default|GetAnimationComponent)) "NewEnumerator0"))))

(event Input|GamepadEvents|GamepadSpecialRight
  (params (Key :type Key%20Structure :default "None"))
  ;[1 1 1] Open Menu
  ;;[1 1 1] Main Menu
  (:Pressed
    (CallFunction|PlayBookAnimation)))

(fn ConstructionScript)

(fn NPCCheck
  (for _array_element (Collision|GetOverlappingActors "/Script/Engine.Actor" :!class /Script/Engine.Actor)
    (Utilities|IsValid (Actor|GetComponentbyClass _array_element "/Game/Character/NPC/NPC.NPC_C")
      (:Is%20Valid
        (return (Actor|GetComponentbyClass _array_element "/Game/Character/NPC/NPC.NPC_C")))))
  (return (Actor|GetComponentbyClass _array_element "/Game/Character/NPC/NPC.NPC_C")))

(fn SetBoxRotationAroundPlayer
  (bind _paper2dactor (Variables|Default|GetPaper2DActor))
  (bind _paper2dactor_2 (Variables|Default|GetPaper2DActor))
  (bind _directionality (Variables|/Game/BluePrints/Components/Paper2DActor.Paper2DActor_C|GetDirectionality _paper2dactor))
  (bind _directionality_2 (Variables|/Game/BluePrints/Components/Paper2DActor.Paper2DActor_C|GetDirectionality _paper2dactor_2))
  (if (not (and (== (.x _directionality) 0.0) (== (.y _directionality) 0.0)))
    (Transformation|SetRelativeRotation (Variables|Default|GetBoxHolder) (Math|Rotator|MakeRotfromZ (Math|Vector|MakeVector (* -1.0 (.x _directionality_2)) (.y _directionality_2) 0.0)) false false)))

(fn IfOverlappingNPC
  (params (Other%20Actor :type Actor%20Object%20Reference) (Other%20Comp :type Actor%20Component%20Object%20Reference))
  (if (Utilities|IsValid (Actor|GetComponentbyClass Other%20Actor "/Game/Character/NPC/NPC.NPC_C"))
    (if (Components|ComponentHasTag Other%20Comp "PromptCollision")
      (Variables|Default|SetIsInInteractBox true))))

(fn NPCLeavesOverlap
  (params (Other%20Actor :type Actor%20Object%20Reference) (Other%20Comp :type Actor%20Component%20Object%20Reference))
  (if (Utilities|IsValid (Actor|GetComponentbyClass Other%20Actor "/Game/Character/NPC/NPC.NPC_C"))
    (if (Components|ComponentHasTag Other%20Comp "PromptCollision")
      (Variables|Default|SetIsInInteractBox false))))

(fn OpenPlayerMenu
  (params (Init%20Key :type Key%20Structure :default "None"))
  (bind _returnvalue (UserInterface|CreateWidget "/Game/BluePrints/UI_Widgets/Menus/Journal/Backdrop/JournalBackdrop.JournalBackdrop_C"))
  (bind _output_get (Variables|Default|SetPlayer%20Menu _returnvalue))
  (Default|FindInitialPage _output_get Init%20Key)
  (UserInterface|Viewport|AddtoViewport _output_get 0))

(fn CreateHUD
  (bind _returnvalue (UserInterface|CreateWidget "/Game/BluePrints/UI_Widgets/HUDS/PlayerHUD/PlayerHUDWidget.PlayerHUDWidget_C" (Game|GetPlayerController 0)))
  (bind _output_get (Variables|Default|SetHUD _returnvalue))
  (UserInterface|Viewport|AddtoViewport _output_get 0))

(fn AttackMovement
  (if (not (Variables|Default|GetNoAttackMoving))
    (CallFunction|AttackMovementUpdate)))

(fn IsinAnimation
  (if (Variables|Default|GetIsAttacking)
    _
    (elif (Variables|Default|GetIsOpeningBook)
      _
      (elif (Variables|Default|GetIsClosingBook)
        _
        (else
          (return true)))))
  (return false))

(fn PushMoveForward
  (params (X :type Float%20%28single-precision%29) (Y :type Float%20%28single-precision%29))
  (bind _paper2dactor (Variables|Default|GetPaper2DActor))
  (bind _directionality (Variables|/Game/BluePrints/Components/Paper2DActor.Paper2DActor_C|GetDirectionality _paper2dactor))
  (bind _returnvalue (Math|Float|Absolute(Float) (.y _directionality)))
  (bind _returnvalue_2 (Math|Float|Absolute(Float) (.x _directionality)))
  (bind _returnvalue_3 (+ _returnvalue_2 _returnvalue))
  (Class|MovementComponent|MoveUpdatedComponent (Variables|Character|GetCharacterMovement) (Math|Vector|MakeVector (* Y (/ (.y _directionality) _returnvalue_3)) (* (/ (.x _directionality) _returnvalue_3) X) 0.0) "0, 0, 0" true))

(fn PlayBookAnimation
  (bind _canpass (CallFunction|IsinAnimation))
  (if _canpass
    (Components|Movement|StopMovementImmediately (Variables|Character|GetCharacterMovement))
    (Class|PaperZDAnimInstance|JumptoNode (Variables|/Script/PaperZD.PaperZDAnimationComponent|GetAnimInstance (Variables|Default|GetAnimationComponent)) "Book" "None")
    (return true)
    (else
      (return false))))

(fn PlayAttackAnimation
  (Class|BPIComboRequest|RequestCombo(Message) (Variables|/Script/PaperZD.PaperZDAnimationComponent|GetAnimInstance (Variables|Default|GetAnimationComponent)) "NewEnumerator0"))

(fn CreateSwipeParticle
  (if (>= (.x (Variables|/Game/BluePrints/Components/Paper2DActor.Paper2DActor_C|GetDirectionality (Variables|Default|GetPaper2DActor))) 0.0)
    (Variables|Default|SetSwipeParticleRotation "0, 0, 0")
    (else
      (Variables|Default|SetSwipeParticleRotation "0,180.000000,0.000000")))
  (Game|SpawnActorfromClass "/Game/BluePrints/Assets/ParticleEffects/Blueprints/BP_SwipeParticle.BP_SwipeParticle_C" (Math|Transform|MakeTransform (Transformation|GetWorldLocation (Variables|Default|GetBoxCollision)) (Variables|Default|GetSwipeParticleRotation) "1,1,1") "Undefined" 0 0)
  (return))

(fn BasicAttack
  (Default|EventAttack (Variables|Default|GetBPC_CMB_AttackComponent) (Variables|/Game/BluePrints/Components/Paper2DActor.Paper2DActor_C|GetDirectionality (Variables|Default|GetPaper2DActor)) "/Game/BluePrints/CombatSystems/WeaponData/WDT_Sword.WDT_Sword"))