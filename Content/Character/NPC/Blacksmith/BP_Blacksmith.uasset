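; Blacksmith NPC Blueprint that shows an interaction prompt when the player comes near.
; Capsule begin and end overlap events pass the overlapping actor, the player character and the E prompt to its NPC object, which handles showing and hiding the prompt.
; The construction script copies the blacksmith's dialogue into that NPC object.
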(event OnComponentBeginOverlap(CapsuleComponent)
  (params (OverlappedComponent :type Primitive%20Component%20Object%20Reference) (OtherActor :type Actor%20Object%20Reference) (OtherComp :type Primitive%20Component%20Object%20Reference) (OtherBodyIndex :type Integer) (bFromSweep :type Boolean) (SweepResult :type Hit%20Result%20Structure%20%28by%20ref%29))
  ;[1 1 1] On EventOverlap for Blacksmith. Checks if player can interact with it. It will check for if NPC is infront of player. If yes, turns on E Prompt. When it leaves, it turns off.
  (Default|InteractionStartOverlap (Variables|Default|GetNPC) OtherActor (Game|GetPlayerCharacter 0) (Variables|Default|GetE_Prompt)))

(event OnComponentEndOverlap(CapsuleComponent)
  (params (OverlappedComponent :type Primitive%20Component%20Object%20Reference) (OtherActor :type Actor%20Object%20Reference) (OtherComp :type Primitive%20Component%20Object%20Reference) (OtherBodyIndex :type Integer))
  ;[1 1 1] On EventOverlap for Blacksmith. Checks if player can interact with it. It will check for if NPC is infront of player. If yes, turns on E Prompt. When it leaves, it turns off.
  (Default|InteractionEndOverlap (Variables|Default|GetNPC) OtherActor (Game|GetPlayerCharacter 0) (Variables|Default|GetE_Prompt)))

(event EventBeginPlay)

(event Collision|EventActorBeginOverlap
  (params (OtherActor :type Actor%20Object%20Reference)))

(event EventTick
  (params (DeltaSeconds :type Float%20%28single-precision%29)))

(fn ConstructionScript
  (Variables|/Game/Character/NPC/NPC.NPC_C|SetNPCDialogue (Variables|Default|GetNPC) (Variables|Default|GetNPCDialogue)))