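; Template 2D PaperZD NPC character with movement-driven directionality and player interaction prompts.
; Tick locks the sprite's world rotation and, while moving, writes the normalized velocity to the NPC component's Directionality.
; BeginPlay hands the dialogue to that component, and capsule overlaps call its interaction start and end functions with the E prompt.
; On destruction, it spawns a death particle actor at its spawn point.
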(event OnComponentBeginOverlap(CapsuleComponent)
  (params (OverlappedComponent :type Primitive%20Component%20Object%20Reference) (OtherActor :type Actor%20Object%20Reference) (OtherComp :type Primitive%20Component%20Object%20Reference) (OtherBodyIndex :type Integer) (bFromSweep :type Boolean) (SweepResult :type Hit%20Result%20Structure%20%28by%20ref%29))
  ;[1 1 1] On EventOverlap for Blacksmith. Checks if player can interact with it. It will check for if NPC is infront of player. If yes, turns on E Prompt. When it leaves, it turns off.
  (Default|InteractionStartOverlap (Variables|Default|GetNPC) OtherActor (Game|GetPlayerCharacter 0) (Variables|Default|GetE_Prompt)))

(event OnComponentEndOverlap(CapsuleComponent)
  (params (OverlappedComponent :type Primitive%20Component%20Object%20Reference) (OtherActor :type Actor%20Object%20Reference) (OtherComp :type Primitive%20Component%20Object%20Reference) (OtherBodyIndex :type Integer))
  ;[1 1 1] On EventOverlap for Blacksmith. Checks if player can interact with it. It will check for if NPC is infront of player. If yes, turns on E Prompt. When it leaves, it turns off.
  (Default|InteractionEndOverlap (Variables|Default|GetNPC) OtherActor (Game|GetPlayerCharacter 0) (Variables|Default|GetE_Prompt)))

(event EventBeginPlay
  (Variables|/Game/Character/NPC/NPC.NPC_C|SetNPCDialogue (Variables|Default|GetNPC) (Variables|Default|GetNPCDialogue)))

(event EventDestroyed
  ;[1 1 1] Spawn particles on death
  (Game|SpawnActorfromClass "/Game/BluePrints/Assets/ParticleEffects/Blueprints/BP_DeathParticle.BP_DeathParticle_C" (Math|Conversions|ToTransform(Vector) (Transformation|GetWorldLocation (Variables|Default|GetSpawnPoint))) "AlwaysSpawn" 0 0))

(event EventTick
  (params (DeltaSeconds :type Float%20%28single-precision%29))
  (bind _charactermovement (Variables|Character|GetCharacterMovement))
  (bind _returnvalue (Pawn|Components|CharacterMovement|GetLastUpdateVelocity _charactermovement))
  (bind _returnvalue_2 (Math|Vector|Normalize _returnvalue))
  ;[1 1 1] PaperZD Actor
  (Transformation|SetWorldRotation (Variables|Default|GetSprite) "0,90.000000, 0" false false) ; Always face same direction
  (bind _output_get (Variables|Default|SetIsMoving (> (Math|Vector|VectorLength _returnvalue) 0.0)))
  (if _output_get ; Only set directionality when moving
    (Variables|/Game/BluePrints/Components/Paper2DActor.Paper2DActor_C|SetDirectionality (Variables|Default|GetNPC) (Math|Vector2D|MakeVector2D (.y _returnvalue_2) (.x _returnvalue_2)))))

(fn ConstructionScript)