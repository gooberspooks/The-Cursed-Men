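; BP_Boar is a PaperZD 2D boar enemy with component-driven health, attack and animation.
; Each tick it locks the sprite's world rotation and, while moving, sets directionality from normalized velocity with X and Y swapped.
; Its attack event passes that direction to the attack component and jumps the Locomotion state machine to Attacking.
; The health component's death event destroys the actor, and destruction spawns a death particle.
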(event Custom|EventKilled
  (params (Instigator :type Actor%20Object%20Reference))
  ;[1 1 1] Destroy on death
  (if (== Instigator self)
    (Actor|DestroyActor)))

(event Custom|EventAttackPlayer
  ;[1 1 1] Attack function
  (Default|EventAttack (Variables|Default|GetBPC_CMB_AttackComponent) (Variables|/Game/BluePrints/Components/Paper2DActor.Paper2DActor_C|GetDirectionality (Variables|Default|GetEnemy)))
  (Class|PaperZDAnimInstance|JumptoNode (Variables|/Script/PaperZD.PaperZDAnimationComponent|GetAnimInstance (Variables|Default|GetAnimationComponent)) "Attacking" "Locomotion"))

(event EventBeginPlay
  ;[1 1 1] Bind on play
  (EventDispatchers|BindEventtoEventonDeath (Variables|Default|GetBPC_CMB_HealthComponent) (delegate Custom|EventKilled)))

(event EventDestroyed
  ;[1 1 1] Spawn particles on death
  (Game|SpawnActorfromClass "/Game/BluePrints/Assets/ParticleEffects/Blueprints/BP_DeathParticle.BP_DeathParticle_C" (Math|Conversions|ToTransform(Vector) (Transformation|GetWorldLocation (Variables|Default|GetSpawnPoint))) "AlwaysSpawn" 0 0))

(event EventTick
  (params (DeltaSeconds :type Float%20%28single-precision%29))
  (bind _charactermovement (Variables|Character|GetCharacterMovement))
  (bind _returnvalue (Pawn|Components|CharacterMovement|GetLastUpdateVelocity _charactermovement))
  (bind _returnvalue_2 (Math|Vector|Normalize _returnvalue))
  ;[1 1 1] PaperZD Actor
  (Transformation|SetWorldRotation (Variables|Default|GetSprite) "0,90.000000, 0" false false) ; Always face same direction
  (bind _output_get (Variables|Default|SetIsMoving (> (Math|Vector|VectorLength _returnvalue) 0.0)))
  (if _output_get ; Only set directionality when moving
    (Variables|/Game/BluePrints/Components/Paper2DActor.Paper2DActor_C|SetDirectionality (Variables|Default|GetEnemy) (Math|Vector2D|MakeVector2D (.y _returnvalue_2) (.x _returnvalue_2)))))

(fn ConstructionScript)