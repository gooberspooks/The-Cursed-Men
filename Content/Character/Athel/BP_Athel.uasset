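; Athel is the player character, a Paper2D-style pawn that walks, talks to NPCs and opens the player menu.
; Axis input drives movement and facing Directionality, which Tick uses to rotate BoxHolder and its collision box around the player.
; That box flags overlaps with NPC prompt collisions, while E or gamepad talks to an NPC component found among overlapping actors.
; Escape creates the menu widget, and 1 debug-prints the inventory.
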(event OnComponentBeginOverlap(BoxCollision)
  (params (OverlappedComponent :type Primitive%20Component%20Object%20Reference) (OtherActor :type Actor%20Object%20Reference) (OtherComp :type Primitive%20Component%20Object%20Reference) (OtherBodyIndex :type Integer) (bFromSweep :type Boolean) (SweepResult :type Hit%20Result%20Structure%20%28by%20ref%29))
  ;[1 1 1] BeginOverlap of BoxCollision to check if overlapping actor is NPC and has PromptCollision tag on a component. If yes, sets InteractBox to on. When it leaves, turns off.
  (CallFunction|IfOverlappingNPC OtherActor OtherComp))

(event OnComponentEndOverlap(BoxCollision)
  (params (OverlappedComponent :type Primitive%20Component%20Object%20Reference) (OtherActor :type Actor%20Object%20Reference) (OtherComp :type Primitive%20Component%20Object%20Reference) (OtherBodyIndex :type Integer))
  ;[1 1 1] BeginOverlap of BoxCollision to check if overlapping actor is NPC and has PromptCollision tag on a component. If yes, sets InteractBox to on. When it leaves, turns off.
  (CallFunction|NPCLeavesOverlap OtherActor OtherComp))

(event EventBeginPlay)

(event Collision|EventActorBeginOverlap
  (params (OtherActor :type Actor%20Object%20Reference)))

(event EventTick
  (params (DeltaSeconds :type Float%20%28single-precision%29))
  ;[1 1 1] Rotates BoxHolder to orient BoxCollision around the player. (exists to check what's infront of player)
  (CallFunction|SetBoxRotationAroundPlayer))

(event Input|AxisEvents|InputAxisMoveRight
  (params (AxisValue :type Float%20%28single-precision%29))
  ;[1 1 1] Controls Character Movement and passes IsHoldingMove = true while running.
  (Variables|Default|SetIsHoldingMove true)
  (Pawn|Input|AddMovementInput (Math|Vector|GetRightVector (Pawn|GetControlRotation :!class /Script/Engine.Pawn)) AxisValue false)
  ;[1 1 1] Checks If Character is moving in any direction before passing to Set IsHoldingMove = false
  (if (== AxisValue 0.0)
    (if (== (stale Input|AxisEvents|InputAxisMoveUp AxisValue) 0.0)
      (Variables|Default|SetIsHoldingMove false)
      (else
        (Variables|/Game/BluePrints/Components/Paper2DActor.Paper2DActor_C|SetDirectionality (Variables|Default|GetPaper2DActor) (Math|Vector2D|MakeVector2D AxisValue (stale Input|AxisEvents|InputAxisMoveUp AxisValue)) :!label _label)))
    (else
      (goto _label))))

(event Input|AxisEvents|InputAxisMoveUp
  (params (AxisValue :type Float%20%28single-precision%29))
  ;[1 1 1] Controls Character Movement and passes IsHoldingMove = true while running.
  (Variables|Default|SetIsHoldingMove true)
  (Pawn|Input|AddMovementInput (Math|Vector|GetForwardVector (Pawn|GetControlRotation :!class /Script/Engine.Pawn)) AxisValue false)
  ;[1 1 1] Checks If Character is moving in any direction before passing to Set IsHoldingMove = false
  (if (== (stale Input|AxisEvents|InputAxisMoveRight AxisValue) 0.0)
    (if (== AxisValue 0.0)
      (Variables|Default|SetIsHoldingMove false)
      (else
        (Variables|/Game/BluePrints/Components/Paper2DActor.Paper2DActor_C|SetDirectionality (Variables|Default|GetPaper2DActor) (Math|Vector2D|MakeVector2D (stale Input|AxisEvents|InputAxisMoveRight AxisValue) AxisValue) :!label _label)))
    (else
      (goto _label))))

(event Input|KeyboardEvents|E
  (params (Key :type Key%20Structure :default "None"))
  (bind _self self)
  ;[1 1 1] Checks If NPC Actor is within range to talk after pressing E Key.
  (:Pressed
    (bind _returnvalue (CallFunction|NPCCheck))
    (Utilities|IsValid _self
      (:Is%20Valid
        (Default|Talk _returnvalue _self)))))

(event Input|GamepadEvents|GamepadFaceButtonLeft
  (params (Key :type Key%20Structure :default "None"))
  (bind _self self)
  ;[1 1 1] Checks If NPC Actor is within range to talk after pressing E Key.
  (:Pressed
    (bind _returnvalue (CallFunction|NPCCheck))
    (Utilities|IsValid _self
      (:Is%20Valid
        (Default|Talk _returnvalue _self)))))

(event Input|KeyboardEvents|1
  (params (Key :type Key%20Structure :default "None"))
  (:Pressed
    (Default|DEBUGPrintContents (Variables|Default|GetInventory))))

(event Input|KeyboardEvents|Escape
  (params (Key :type Key%20Structure :default "None"))
  (:Pressed
    (CallFunction|OpenPlayerMenu)))

(fn ConstructionScript)

(fn NPCCheck
  (for _array_element (Collision|GetOverlappingActors "/Script/Engine.Actor" :!class /Script/Engine.Actor)
    (Utilities|IsValid (Actor|GetComponentbyClass _array_element "/Game/BluePrints/Components/NPC.NPC_C")
      (:Is%20Valid
        (return (Actor|GetComponentbyClass _array_element "/Game/BluePrints/Components/NPC.NPC_C")))))
  (return (Actor|GetComponentbyClass _array_element "/Game/BluePrints/Components/NPC.NPC_C")))

(fn SetBoxRotationAroundPlayer
  (bind _paper2dactor (Variables|Default|GetPaper2DActor))
  (bind _directionality (Variables|/Game/BluePrints/Components/Paper2DActor.Paper2DActor_C|GetDirectionality _paper2dactor))
  (Transformation|SetRelativeRotation (Variables|Default|GetBoxHolder) (Math|Rotator|MakeRotfromZ (Math|Vector|MakeVector (* -1.0 (.x _directionality)) (.y _directionality) 0.0)) false false))

(fn IfOverlappingNPC
  (params (Other%20Actor :type Actor%20Object%20Reference) (Other%20Comp :type Actor%20Component%20Object%20Reference))
  (if (Utilities|IsValid (Actor|GetComponentbyClass Other%20Actor "/Game/BluePrints/Components/NPC.NPC_C"))
    (if (Components|ComponentHasTag Other%20Comp "PromptCollision")
      (Variables|Default|SetIsInInteractBox true))))

(fn NPCLeavesOverlap
  (params (Other%20Actor :type Actor%20Object%20Reference) (Other%20Comp :type Actor%20Component%20Object%20Reference))
  (if (Utilities|IsValid (Actor|GetComponentbyClass Other%20Actor "/Game/BluePrints/Components/NPC.NPC_C"))
    (if (Components|ComponentHasTag Other%20Comp "PromptCollision")
      (Variables|Default|SetIsInInteractBox false))))

(fn OpenPlayerMenu
  (bind _returnvalue (UserInterface|CreateWidget "/Game/BluePrints/UI_Widgets/Menus/PlayerMenuWidget.PlayerMenuWidget_C"))
  (UserInterface|Viewport|AddtoViewport _returnvalue 0))