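; Base AI pawn that wanders to random reachable points and picks a random behavior when the player enters its SphereOfInfluence.
; An integer CurrentBehavior selects wander, stare, follow or attack; attack is unimplemented and falls back to wandering.
; Stare stops movement and turns smoothly toward the player on Tick until the player leaves.
; Follow uses AIMoveTo, randomly repeating on arrival, with a random-length timer that cancels back to wandering.
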(event OnComponentBeginOverlap(SphereOfInfluence)
  (params (OverlappedComponent :type Primitive%20Component%20Object%20Reference) (OtherActor :type Actor%20Object%20Reference) (OtherComp :type Primitive%20Component%20Object%20Reference) (OtherBodyIndex :type Integer) (bFromSweep :type Boolean) (SweepResult :type Hit%20Result%20Structure%20%28by%20ref%29))
  ;[1 1 1] Chose Behavior on Player Overlap
  (if (== OtherActor (Game|GetPlayerCharacter 0))
    (bind _output_get (Variables|Default|SetCurrentBehavior (Math|Random|RandomInteger 4)))
    (switch int _output_get
      (:Default
        (CallFunction|Wander :!label _label))
      (:0
        (goto _label))
      (:1
        (CallFunction|Stare))
      (:2
        (CallFunction|FollowPlayer))
      (:3
        (CallFunction|AttackPlayer)))))

(event Custom|Wander
  (bind _returnvalue (Math|Random|RandomFloatinRange 1.0 7.0))
  ;[1 1 1] Wander
  (if (== (Variables|Default|GetCurrentBehavior) 0)
    (bind _output_get (Variables|Default|SetTargetLocation (.RandomLocation (AI|Navigation|GetRandomReachablePointinRadius (Transformation|GetActorLocation) 2.5e+03 0 0))))
    (AI|AIMoveTo self _output_get 0 5.0 false
      (:OnSuccess
        (Utilities|FlowControl|Delay _returnvalue)
        (CallFunction|Wander))
      (:OnFail
        (Utilities|FlowControl|Delay _returnvalue)
        (CallFunction|Wander)))))

(event Custom|AttackPlayer
  ;[1 1 1] Attack Player (Not Implemented)
  (Variables|Default|SetCurrentBehavior 0)
  (CallFunction|Wander))

(event Custom|Stare
  ;[1 1 1] Stare At Player
  (AI|Navigation|StopMovement (AI|GetAIController self))
  (Utilities|FlowControl|Delay (Math|Random|RandomFloatinRange 0.5 5.0) :!label _label)
  (if (Collision|IsOverlappingActor (Variables|Default|GetSphereOfInfluence) (Game|GetPlayerCharacter 0) :!class /Script/Engine.PrimitiveComponent)
    (goto _label)
    (else
      (Variables|Default|SetCurrentBehavior 0)
      (CallFunction|Wander))))

(event Custom|FollowPlayer
  ;[1 1 1] Follow Player
  (Utilities|Time|SetTimerbyFunctionName 0 "CancelFollow" (Math|Random|RandomFloatinRange 3.0 1e+01))
  (Variables|Default|SetFollowingPlayer true)
  (AI|AIMoveTo self "0, 0, 0" (Game|GetPlayerCharacter 0) 1e+01 true
    (:OnSuccess
      (Variables|Default|SetFollowingPlayer true)
      (Utilities|FlowControl|Delay 1.0)
      (if (Math|Random|RandomBool)
        (CallFunction|FollowPlayer)
        (else
          (Variables|Default|SetCurrentBehavior 0)
          (CallFunction|Wander))))))

(event EventBeginPlay
  ;[1 1 1] Wander on Start
  (Utilities|FlowControl|Delay (Math|Random|RandomFloatinRange 0.0 5.0))
  (CallFunction|Wander))

(event EventTick
  (params (DeltaSeconds :type Float%20%28single-precision%29))
  ;[1 1 1] Event Tick
  (switch int (Variables|Default|GetCurrentBehavior)
    (:1
      (CallFunction|RotateTowardsPlayer))))

(fn ConstructionScript)

(fn RotateTowardsPlayer
  (Transformation|SetActorRotation (Math|Interpolation|RInterpTo (Transformation|GetActorRotation) (Math|Rotator|FindLookatRotation (Transformation|GetActorLocation) (Transformation|GetActorLocation (Game|GetPlayerCharacter 0))) (Utilities|Time|GetWorldDeltaSeconds) 2.0)))

(fn CancelFollow
  (if (Variables|Default|GetFollowingPlayer)
    (AI|Navigation|StopMovement (AI|GetAIController self))
    (Variables|Default|SetCurrentBehavior 0)
    (CallFunction|Wander)))