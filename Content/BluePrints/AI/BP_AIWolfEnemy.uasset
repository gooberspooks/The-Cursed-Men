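; BP_AIWolfEnemy is an AI-controlled wolf enemy that can share its aggro target with the rest of its pack.
; AlertPack reads TargetActor from this wolf's blackboard and passes it to EventDrawnAggro on the AIC_WolfEnemy controller of each wolf in PackMembers.
; The file holds no other active logic beyond a parent construction script call, and AlertPack is not called within it.
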(event Custom|AlertPack
  ;[1 1 1] Set target actor for other wolves in pack
  (for _array_element (Variables|Default|GetPackMembers)
    (bind _asaic_wolf_enemy (Utilities|Casting|CastToAIC_WolfEnemy (AI|GetAIController _array_element)))
    (Default|EventDrawnAggro _asaic_wolf_enemy (AI|Components|Blackboard|GetValueasObject (AI|GetBlackboard (AI|GetAIController self)) (Utilities|Name|MakeLiteralName "TargetActor")))))

(event EventBeginPlay
  (|CallParentFunction) ; This node is disabled and will not be called.\nDrag off pins to build functionality.
)

(event Collision|EventActorBeginOverlap
  (params (OtherActor :type Actor%20Object%20Reference)))

(event EventTick
  (params (DeltaSeconds :type Float%20%28single-precision%29))
  (|CallParentFunction DeltaSeconds) ; This node is disabled and will not be called.\nDrag off pins to build functionality.
)

(fn ConstructionScript
  (|CallParentFunction))