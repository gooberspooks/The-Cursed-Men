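; AIC_Base is an AI controller that runs the BHT_Boar behavior tree and feeds its blackboard from damage and perception events.
; On BeginPlay it starts the tree and binds to the controlled pawn's damage event, which sets the AIDamaged key to true.
; Perception updates for the player character write it to TargetActor, without checking whether it was sensed or lost.
; Neither key is cleared in this controller.
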(event OnTargetPerceptionUpdated(AIPerception)
  (params (Actor :type Actor%20Object%20Reference) (Stimulus :type AI%20Stimulus%20Structure))
  (if (== Actor (Game|GetPlayerCharacter 0))
    (AI|Components|Blackboard|SetValueasObject (Variables|Default|GetBlackboard) (Utilities|Name|MakeLiteralName "TargetActor") Actor)))

(event Custom|EventTakenDamage
  (params (DamagedActor :type Actor%20Object%20Reference) (Damage :type Float%20%28single-precision%29) (DamageType :type Damage%20Type%20Object%20Reference) (InstigatedBy :type Controller%20Object%20Reference) (DamageCauser :type Actor%20Object%20Reference))
  (AI|Components|Blackboard|SetValueasBool (Variables|Default|GetBlackboard) (Utilities|Name|MakeLiteralName "AIDamaged") true))

(event EventBeginPlay
  (AI|RunBehaviorTree "/Game/BluePrints/AI/BHT_Boar.BHT_Boar")
  (EventDispatchers|AssignOnTakeAnyDamage (Pawn|GetControlledPawn) (delegate Custom|EventTakenDamage)))

(fn ConstructionScript)