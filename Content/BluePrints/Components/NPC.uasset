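; NPC component that lets the player character, BP_Athel, talk to its owning character.
; Overlap functions show or hide an interaction prompt and track whether the player is in range, requiring the player to be inside their interact box on entry.
; Talk checks that range flag, sets a 2D Directionality from the owner-to-player direction so the NPC faces the player, then begins its NPCDialogue.
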(event EventBeginPlay)

(event EventTick
  (params (DeltaSeconds :type Float%20%28single-precision%29)))

(fn Talk
  (params (Interacter :type Actor%20Object%20Reference))
  ;[1 1 1] Checks if player is in Interact Range.
  (if (Variables|Default|GetisInInteractRange)
    (bind _asbp_athel (Utilities|Casting|CastToBP_Athel Interacter))
    (Utilities|IsValid _asbp_athel
      (:Is%20Valid
        ;[1 1 1] Gets location of both player and owner. Uses it to change the way owner is facing to look at player.
        (Variables|Default|SetDirectionality (Math|Vector2D|MakeVector2D (.y (Math|Vector|Normalize (- (Transformation|GetActorLocation _asbp_athel) (Transformation|GetActorLocation (Components|GetOwner))))) (.x (Math|Vector|Normalize (- (Transformation|GetActorLocation _asbp_athel) (Transformation|GetActorLocation (Components|GetOwner)))))))
        (Utilities|IsValid (Variables|Default|GetNPCDialogue)
          (:Is%20Valid
            (Default|BeginDialogue (Variables|Default|GetNPCDialogue))))))))

(fn InteractionStartOverlap
  (params (OtherActor :type Actor%20Object%20Reference) (Player%20Character :type Actor%20Object%20Reference) (Prompt :type Paper%20Sprite%20Component%20Object%20Reference))
  (if (== OtherActor Player%20Character)
    (bind _asbp_athel (Utilities|Casting|CastToBP_Athel OtherActor))
    (if (Variables|/Game/Character/Athel/BP_Athel.BP_Athel_C|GetIsInInteractBox _asbp_athel)
      (Rendering|SetVisibility Prompt true true)
      (Variables|Default|SetisInInteractRange true))))

(fn InteractionEndOverlap
  (params (Other%20Actor :type Actor%20Object%20Reference) (Player%20Character :type Actor%20Object%20Reference) (Prompt :type Paper%20Sprite%20Component%20Object%20Reference))
  (if (== Other%20Actor Player%20Character)
    (Rendering|SetVisibility Prompt false true)
    (Variables|Default|SetisInInteractRange false)))