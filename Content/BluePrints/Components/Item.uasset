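; Item component that identifies its owning actor as an inventory item through an item row handle and quantity.
; On BeginPlay it runs playtest logic, marked as deletable, that adds the item to the BP_Athel player's Inventory after a short delay.
; If a slot for it is found, it later calls RemoveItem without removing the whole stack.
; It then destroys the owning actor if the Item_Data row allows discarding.
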(event EventBeginPlay
  (bind _itemid (Variables|Default|GetItemID))
  ;[1 1 1] For playtesting add and remove item features. (Can delete when in actual use)
  (Utilities|FlowControl|Delay 1.0)
  (bind _asbp_athel (Utilities|Casting|CastToBP_Athel (Game|GetPlayerCharacter 0)))
  (Utilities|IsValid (Variables|/Game/Character/Athel/BP_Athel.BP_Athel_C|GetInventory _asbp_athel)
    (:Is%20Valid
      (bind _success (Default|AddItem (Variables|/Game/Character/Athel/BP_Athel.BP_Athel_C|GetInventory _asbp_athel) (.rowname _itemid) (Variables|Default|GetQuantity)))
      (if _success
        (bind (_index _foundslot) (Default|FindSlot (Variables|/Game/Character/Athel/BP_Athel.BP_Athel_C|GetInventory _asbp_athel) (.rowname _itemid)))
        (if _foundslot
          (Utilities|FlowControl|Delay 5.0)
          (Default|RemoveItem (Variables|/Game/Character/Athel/BP_Athel.BP_Athel_C|GetInventory _asbp_athel) _index false false)
          (bind _returnvalue (Utilities|GetDataTableRow "/Game/BluePrints/Items/Item_Data.Item_Data" (.rowname _itemid))
            (:then
              (if (.candiscard _returnvalue)
                (Actor|DestroyActor (Components|GetOwner))))))))))

(event EventTick
  (params (DeltaSeconds :type Float%20%28single-precision%29))
  ;[1 1 1] For playtesting add and remove item features. (Can delete when in actual use)
)