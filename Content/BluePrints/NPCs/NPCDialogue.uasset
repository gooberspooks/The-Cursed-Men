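; NPC dialogue Blueprint that plays a bilingual English/Spanish conversation from a data table in a Dialogue widget.
; BeginDialogue opens the widget with the mouse cursor and passes itself in; AdvanceText displays the row at RowNumber, which is not incremented here.
; Rows set speaker and language-specific text and words, though only English text is pushed to the widget.
; A missing row or changed DialogueID closes the widget and resets state.
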(event Custom|AdvanceText
  (CallFunction|DisplayDialogue))

(event Custom|BeginDialogue
  (bind _returnvalue (Game|GetPlayerController 0))
  (bind _returnvalue_2 (UserInterface|CreateWidget "/Game/BluePrints/UI_Widgets/TextBox/Dialogue.Dialogue_C" _returnvalue))
  (Variables|Default|SetDialogueCache _returnvalue_2)
  (UserInterface|Viewport|AddtoViewport _returnvalue_2 0)
  (Variables|/Script/Engine.PlayerController|SetbShowMouseCursor _returnvalue true)
  (Variables|/Game/BluePrints/UI_Widgets/TextBox/Dialogue.Dialogue_C|SetDialogueBlueprint _returnvalue_2 self)
  (CallFunction|DisplayDialogue))

(event Custom|EndDialogue
  (Widget|RemovefromParent (Variables|Default|GetDialogueCache))
  (Variables|/Script/Engine.PlayerController|SetbShowMouseCursor (Game|GetPlayerController 0) false)
  (Variables|Default|SetRow%20Number (Variables|Default|GetRow%20Number%20Initial))
  (Variables|Default|SetDialogue%20ID -1)
  (Variables|Default|SetCharacter%20Name "None")
  (Variables|Default|SetInEnglish false)
  (Variables|Default|SetDialogue "")
  (Variables|Default|SetWords ""))

(event EventBeginPlay
  (Variables|Default|SetRow%20Number%20Initial (Variables|Default|GetRow%20Number)))

(fn DisplayDialogue
  (bind _returnvalue (Utilities|GetDataTableRow "/Game/BluePrints/DataTables/Dialogue.Dialogue" (Utilities|String|StringToName (Utilities|String|ToString(Integer) (Variables|Default|GetRow%20Number))))
    (:then
      (if (or (== (Variables|Default|GetDialogue%20ID) -1) (== (Variables|Default|GetDialogue%20ID) (.DialogueID (Utilities|Struct|BreakDialogueStructure _returnvalue))))
        (Variables|Default|SetDialogue%20ID (.DialogueID (Utilities|Struct|BreakDialogueStructure _returnvalue)))
        (Variables|Default|SetCharacter%20Name (.CharacterName (Utilities|Struct|BreakDialogueStructure _returnvalue)))
        (Utilities|FlowControl|Sequence
          (:then_0
            (bind _output_get (Variables|Default|SetInEnglish (.InEnglish (Utilities|Struct|BreakDialogueStructure _returnvalue))))
            (if _output_get
              (bind _output_get_2 (Variables|Default|SetDialogue (.EnglishEquivalent (Utilities|Struct|BreakDialogueStructure _returnvalue))))
              (Variables|Default|SetWords (.EnglishWordsandPhrases (Utilities|Struct|BreakDialogueStructure _returnvalue)))
              (Default|SetEnglishText (Variables|Default|GetDialogueCache) (Utilities|Text|ToText(String) _output_get_2))
              (else
                (Variables|Default|SetDialogue (.SpanishDialogue (Utilities|Struct|BreakDialogueStructure _returnvalue)))
                (Variables|Default|SetWords (.SpanishWordsandPhrases (Utilities|Struct|BreakDialogueStructure _returnvalue))))))
          (:then_1
            (if (.PlayerSpeaks (Utilities|Struct|BreakDialogueStructure _returnvalue))
              (Default|SetName (Variables|Default|GetDialogueCache) "Athel")
              (else
                (Default|SetName (Variables|Default|GetDialogueCache) (Utilities|Text|ToText(Name) (Variables|Default|GetCharacter%20Name)))))))
        (else
          (CallFunction|EndDialogue))))
    (:RowNotFound
      (CallFunction|EndDialogue))))