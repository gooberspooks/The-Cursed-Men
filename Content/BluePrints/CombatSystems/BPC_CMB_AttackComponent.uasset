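; Actor component that gives its owner a melee-style attack, damaging whatever lies in the attack direction.
; On BeginPlay it caches the owner and name; Attack sphere-traces from the owner along the direction, with X and Y swapped, up to AttackDistance on Visibility.
; Each hit receives AttackDamage as DT_CMB_True.
; An unconnected branch would spawn BP_CMB_BladeAttack from WeaponData for swords, but never runs.
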(event Custom|Attack
  (params (AttackDirection :type Vector%202D%20Structure))
  (bind (_x _y) (Math|Vector2D|BreakVector2D AttackDirection))
  (bind _owner (Variables|Default|GetOwner))
  (bind _returnvalue (Transformation|GetActorLocation _owner))
  ;[1 1 1] Sphere trace for applying damage
  (bind (_outhits _returnvalue_2) (Collision|MultiSphereTraceByChannel _returnvalue (+ _returnvalue (* (Math|Vector|MakeVector _y _x 0.0) (Variables|Default|GetAttackDistance))) 25.0 "TraceTypeQuery1" false 0 "None"))
  (if _returnvalue_2 ; If hit
    (for _array_element _outhits ; Each actor hit
      (Game|Damage|ApplyDamage (.HitActor (Collision|BreakHitResult _array_element)) (Variables|Default|GetAttackDamage) 0 0 "/Game/BluePrints/CombatSystems/DT_CMB_True.DT_CMB_True_C"))))

(event EventBeginPlay
  (bind _output_get (Variables|Default|SetOwner (Components|GetOwner))) ; Set owner of component
  (Variables|Default|SetActorName (Utilities|GetDisplayName _output_get)) ; Set name of owner
)