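; BP_CMB_BladeAttack is a moving attack hitbox actor in the combat system that damages what it overlaps.
; Tick sweeps it forward along its root's facing at MoveSpeed and destroys it once its lifetime reaches MaxLifetime.
; The Cube's begin overlap applies damage once per actor, using the ActorsHit array to skip repeat hits.
; The construction script scales the Cube to AttackSize.
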(event OnComponentBeginOverlap(Cube)
  (params (OverlappedComponent :type Primitive%20Component%20Object%20Reference) (OtherActor :type Actor%20Object%20Reference) (OtherComp :type Primitive%20Component%20Object%20Reference) (OtherBodyIndex :type Integer) (bFromSweep :type Boolean) (SweepResult :type Hit%20Result%20Structure%20%28by%20ref%29))
  (bind _actorshit (Variables|Default|GetActorsHit))
  (if (not (Utilities|Array|ContainsItem _actorshit OtherActor))
    (Utilities|Array|AddUnique _actorshit OtherActor)
    (Game|Damage|ApplyDamage OtherActor (Variables|Default|GetAttackDamage) 0 0 (Variables|Default|GetDamage%20Type))))

(event EventTick
  (params (DeltaSeconds :type Float%20%28single-precision%29))
  (bind _output_get (Variables|Default|SetCurrentLifetime (+ DeltaSeconds (Variables|Default|GetCurrentLifetime))))
  (if (>= _output_get (Variables|Default|GetMaxLifetime))
    (Actor|DestroyActor)
    (else
      (Transformation|AddActorWorldOffset (* (* (Math|Vector|GetForwardVector (Transformation|GetWorldRotation (Variables|Default|GetDefaultSceneRoot))) (Variables|Default|GetMoveSpeed)) DeltaSeconds) true))))

(fn ConstructionScript
  (Transformation|SetRelativeScale3D (Variables|Default|GetCube) (Variables|Default|GetAttackSize)))