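; Health component for the combat system that tracks its owner's health and defense, flagging whether the owner is the player.
; It binds to the owner's AnyDamage event, nullifies hits while dodging, scales them by a shield percentage while defending, then subtracts flat defense.
; The clamped result reduces health and fires a HealthUpdated event.
; Near-zero health calls HandleDeath, which is an empty stub here.
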(event Custom|OnDamageTaken
  (params (DamagedActor :type Actor%20Object%20Reference) (Damage :type Float%20%28single-precision%29) (DamageType :type Damage%20Type%20Object%20Reference) (InstigatedBy :type Controller%20Object%20Reference) (DamageCauser :type Actor%20Object%20Reference))
  ;[1 1 1] Actions performed upon taken damage
  (bind _calculateddamage (CallFunction|CalculateDamage Damage DamageType))
  (CallFunction|ApplyDamage _calculateddamage)
  (if (Math|Float|NearlyEqual(Float) (Variables|Default|GetCurrentHealthPoints) 0.0 1e-06)
    (CallFunction|HandleDeath)))

(event EventBeginPlay
  ;[1 1 1] Initial variable setup
  (bind _output_get (Variables|Default|SetOwner (Components|GetOwner)))
  (Variables|Default|SetIsPlayer (== _output_get (Game|GetPlayerCharacter 0)))
  (EventDispatchers|AssignOnTakeAnyDamage (Variables|Default|GetOwner) (delegate Custom|OnDamageTaken))
  (Variables|Default|SetCurrentHealthPoints (Variables|Default|GetMaxHealthPoints))
  (Variables|Default|SetCurrentDefense (Variables|Default|GetInitialDefense)))

(fn ApplyDamage
  (params (Damage :type Float%20%28single-precision%29))
  (bind _output_get (Variables|Default|SetCurrentHealthPoints (Math|Float|Clamp(Float) (- (Variables|Default|GetCurrentHealthPoints) Damage) 0.0 (Variables|Default|GetMaxHealthPoints))))
  (Default|CallEventHealthUpdated (Variables|Default|GetIsPlayer) _output_get (Variables|Default|GetMaxHealthPoints))
  (return))

(fn CalculateDamage
  (params (IncomingDamage :type Float%20%28single-precision%29) (DamageType :type Damage%20Type%20Object%20Reference))
  (LocalVariables|SetFinalDamage IncomingDamage)
  (if (Variables|Default|GetIsDodging)
    (LocalVariables|SetFinalDamage 0.0) ; Nullify damage if player has i-frames
    (elif (Variables|Default|GetIsDefending)
      (LocalVariables|SetFinalDamage (* (LocalVariables|GetFinalDamage) (/ (Variables|Default|GetShieldDamageReduction) 1e+02)))))
  (return (Math|Float|Clamp(Float) (- (LocalVariables|GetFinalDamage) (Variables|Default|GetCurrentDefense)) 0.0 (Variables|Default|GetMaxHealthPoints))))

(fn HandleDeath)