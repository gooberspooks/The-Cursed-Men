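; Actor component that performs attacks by spawning a separate world attack actor in a given direction from its owner.
; Attack maps the 2D direction onto the world plane with X and Y swapped, then spawns at AttackDistance, facing away from the owner.
; AttackData supplies the actor class, name, damage, damage type, size, lifetime and speed, with a fixed boost added to speed.
; An older sphere-trace damage path remains as unconnected test code.
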(event Custom|Attack
  (params (AttackDirection :type Vector%202D%20Structure))
  (bind (_x _y) (Math|Vector2D|BreakVector2D AttackDirection))
  (bind _attackdistance (Variables|Default|GetAttackDistance))
  (bind _owner (Variables|Default|GetOwner))
  (bind _returnvalue (Transformation|GetActorLocation _owner))
  (bind _returnvalue_2 (Math|Vector|MakeVector _y _x 0.0))
  (bind _returnvalue_3 (* _returnvalue_2 _attackdistance))
  (bind _returnvalue_4 (+ _returnvalue _returnvalue_3))
  ;[1 1 1] Spawn separate Actor for 3D attack
  (bind (_worldattack _attackname _attackspeed _attackduration _attackdamage _attacksize _damagetype) (Default|GetData (Variables|Default|GetAttackData))) ; Get specs from data type
  (Game|SpawnActorfromClass _worldattack (Math|Transform|MakeTransform _returnvalue_4 (Math|Rotator|FindLookatRotation _returnvalue _returnvalue_4)) "Undefined" 0 _attackname (+ _attackspeed 2e+02) _attackduration _attackdamage _attacksize _damagetype 0) ; Spawn attack
)

(event EventBeginPlay
  (bind _output_get (Variables|Default|SetOwner (Components|GetOwner))) ; Set owner of component
  (Variables|Default|SetActorName (Utilities|GetDisplayName _output_get)) ; Set name of owner
)