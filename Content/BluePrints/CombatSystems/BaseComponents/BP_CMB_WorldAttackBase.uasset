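; Base world attack actor for combat that sweeps forward at MoveSpeed and damages what it overlaps.
; Overlaps skip the instigator and apply AttackDamage once per actor, tracked in ActorsHit.
; Tick destroys it when CurrentLifetime reaches MaxLifetime.
; Construction scales AttackCollision, sets the inversely named TimeLimited to freeze the timer for non-positive lifetimes, then overwrites MaxLifetime with one second in every case.
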(event Collision|EventActorBeginOverlap
  (params (OtherActor :type Actor%20Object%20Reference))
  (bind _actorshit (Variables|Default|GetActorsHit))
  (if (!= OtherActor (Variables|Default|GetInstigatorActor)) ; Making sure actors don't damage themselves
    (if (not (Utilities|Array|ContainsItem _actorshit OtherActor))
      (Utilities|Array|AddUnique _actorshit OtherActor)
      (Game|Damage|ApplyDamage OtherActor (Variables|Default|GetAttackDamage) 0 0 (Variables|Default|GetDamage%20Type)))))

(event EventTick
  (params (DeltaSeconds :type Float%20%28single-precision%29))
  (if (Variables|Default|GetTimeLimited) ; Skip increment time so actor will never kill self
    _
    (else
      (bind _output_get (Variables|Default|SetCurrentLifetime (+ DeltaSeconds (Variables|Default|GetCurrentLifetime))))))
  (if (>= _output_get (Variables|Default|GetMaxLifetime))
    (Actor|DestroyActor)
    (else
      (Transformation|AddActorWorldOffset (* (* (Math|Vector|GetForwardVector (Transformation|GetWorldRotation (Variables|Default|GetDefaultSceneRoot))) (Variables|Default|GetMoveSpeed)) DeltaSeconds) true) ; Moving actor forwards
    )))

(fn ConstructionScript
  (Transformation|SetRelativeScale3D (Variables|Default|GetAttackCollision) (Variables|Default|GetAttackSize))
  (Variables|Default|SetTimeLimited (<= (Variables|Default|GetMaxLifetime) 0.0)) ; Will not kill self if <=0
  (Variables|Default|SetMaxLifetime 1.0) ; Setting Max to non-zero so kill comparison is never true
)