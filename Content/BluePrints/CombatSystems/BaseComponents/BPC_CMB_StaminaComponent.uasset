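; Actor component that tracks stamina for its owner in the combat system, clamped between zero and a maximum.
; A looping timer set on BeginPlay adds one point per tick at a rate set by RegenRate.
; Consuming stamina pauses that timer, and a retriggerable delay resumes it once RegenDelay passes without further consumption.
; Every change, including manual refills, broadcasts the owner's name and stamina values for UI updates.
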(event Custom|EventStaminaConsumed
  (params (AmountConsumed :type Float%20%28single-precision%29))
  (Utilities|Time|PauseTimerbyHandle (Variables|Default|GetStaminaRegenLoop)) ; Pausing regen
  (bind _output_get (Variables|Default|SetCurrentStamina (Math|Float|Clamp(Float) (- (Variables|Default|GetCurrentStamina) AmountConsumed) 0.0 (Variables|Default|GetMaxStamina))))
  (Default|CallEventStaminaUpdated (Variables|Default|GetActorName) _output_get (Variables|Default|GetMaxStamina)) ; Call evnet for UI updates
  (Utilities|FlowControl|RetriggerableDelay (Variables|Default|GetRegenDelay)) ; Delay before regen continues
  (Utilities|Time|UnpauseTimerbyHandle (Variables|Default|GetStaminaRegenLoop)) ; Unpause regen
)

(event EventBeginPlay
  (bind _output_get (Variables|Default|SetOwner (Components|GetOwner))) ; Set component owner
  (Variables|Default|SetActorName (Utilities|GetDisplayName _output_get)) ; Set owner name
  (bind _returnvalue (Utilities|Time|SetTimerbyFunctionName 0 "StaminaRegen" (/ 1.0 (Variables|Default|GetRegenRate)) true)) ; Set function to add back stamina
  (Variables|Default|SetStaminaRegenLoop _returnvalue) ; Setting Timer function as variable for later
)

(fn StaminaRegen
  (bind _output_get (Variables|Default|SetCurrentStamina (Math|Float|Clamp(Float) (+ (Variables|Default|GetCurrentStamina) 1.0) 0.0 (Variables|Default|GetMaxStamina))))
  (Default|CallEventStaminaUpdated (Variables|Default|GetActorName) _output_get (Variables|Default|GetMaxStamina))
  (return))

(fn RefillStamina
  (params (RefillAmount :type Float%20%28single-precision%29))
  (bind _output_get (Variables|Default|SetCurrentStamina (Math|Float|Clamp(Float) (+ RefillAmount (Variables|Default|GetCurrentStamina)) 0.0 (Variables|Default|GetMaxStamina))))
  (Default|CallEventStaminaUpdated (Variables|Default|GetActorName) _output_get (Variables|Default|GetMaxStamina)))