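; BP_DamageArea is a damage volume that hurts overlapping actors on entry and is set up to keep damaging them over time.
; Begin overlap stores the actor, applies InitialDamage and starts a looping timer on DamageTarget at a rate set by DamageSec.
; DamageTarget applies one damage point to its DamagedActor parameter, which the name-based timer does not supply.
; End overlap clears the single timer handle after an actor comparison.
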(event Collision|EventActorBeginOverlap
  (params (OtherActor :type Actor%20Object%20Reference))
  (Variables|Default|SetOther%20Actor OtherActor)
  (Game|Damage|ApplyDamage OtherActor (Variables|Default|GetInitialDamage) 0 0)
  (bind _returnvalue (Utilities|Time|SetTimerbyFunctionName 0 "DamageTarget" (/ 1.0 (Variables|Default|GetDamage/Sec)) true))
  (Variables|Default|SetDamageTimer _returnvalue))

(event Collision|EventActorEndOverlap
  (params (OtherActor :type Actor%20Object%20Reference))
  (if (== OtherActor (Variables|Default|GetOther%20Actor))
    (Utilities|Time|ClearandInvalidateTimerbyHandle (Variables|Default|GetDamageTimer))))

(fn ConstructionScript)

(fn DamageTarget
  (params (DamagedActor :type Actor%20Object%20Reference))
  (Game|Damage|ApplyDamage DamagedActor 1.0 0 0))