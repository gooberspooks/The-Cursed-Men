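; NPC dialogue controller that shows data-table conversations in a Dialogue widget, with Spanish text and word translations.
; BeginDialogue opens the widget; DisplayDialogue loads the row at RowNumber, splitting delimited word lists and setting the speaker name.
; Rows sharing a DialogueID form one conversation; a different ID or missing row closes it and resets state.
; AdvanceText redisplays from RowNumber, which is not incremented here, after placeholder quest and item prints.
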(event Custom|AdvanceText
  (Utilities|FlowControl|Sequence
    (:then_0
      (if (Variables|Default|GetActivateQuest)
        (Development|PrintString "Quest Activated (Temporary String)")))
    (:then_1
      (if (Variables|Default|GetGiveItem)
        (Development|PrintString "Item get (Temporary String)")))
    (:then_2
      (CallFunction|DisplayDialogue))))

(event Custom|BeginDialogue
  (bind _returnvalue (Game|GetPlayerController 0))
  (bind _returnvalue_2 (UserInterface|CreateWidget "/Game/BluePrints/UI_Widgets/Pop-Ups/TextBox/Dialogue.Dialogue_C" _returnvalue))
  (Variables|Default|SetDialogueCache _returnvalue_2)
  (UserInterface|Viewport|AddtoViewport _returnvalue_2 0)
  (Variables|/Script/Engine.PlayerController|SetbShowMouseCursor _returnvalue true)
  (Variables|/Game/BluePrints/UI_Widgets/Pop-Ups/TextBox/Dialogue.Dialogue_C|SetDialogueBlueprint _returnvalue_2 self)
  (CallFunction|DisplayDialogue))

(event Custom|EndDialogue
  (Widget|RemovefromParent (Variables|Default|GetDialogueCache))
  (Variables|/Script/Engine.PlayerController|SetbShowMouseCursor (Game|GetPlayerController 0) false)
  (Variables|Default|SetRow%20Number (Variables|Default|GetRow%20Number%20Initial))
  (Variables|Default|SetCharacterName "None")
  (Variables|Default|SetDialogue%20ID -1)
  (Variables|Default|SetDialogue "")
  (Variables|Default|SetWords "")
  (Variables|Default|SetEquivalentWords "")
  (Variables|Default|SetPlayerSpeaks false)
  (Variables|Default|SetActivateQuest false)
  (Variables|Default|SetGiveItem false))

(event EventBeginPlay
  (Variables|Default|SetRow%20Number%20Initial (Variables|Default|GetRow%20Number)))

(fn DisplayDialogue
  (bind _dialoguecache (Variables|Default|GetDialogueCache))
  (bind _returnvalue (Utilities|GetDataTableRow "/Game/BluePrints/Dialogue/Dialogue.Dialogue" (Utilities|String|StringToName (Utilities|String|ToString(Integer) (Variables|Default|GetRow%20Number))))
    (:then
      ;[1 1 1] If the Dialogue ID is the same or -1, the conversation continues.
      (if (or (== (Variables|Default|GetDialogue%20ID) -1) (== (Variables|Default|GetDialogue%20ID) (.DialogueID (Utilities|Struct|BreakDialogueStructure _returnvalue))))
        (Variables|Default|SetCharacterName (.CharacterName (Utilities|Struct|BreakDialogueStructure _returnvalue)))
        (Variables|Default|SetDialogue%20ID (.DialogueID (Utilities|Struct|BreakDialogueStructure _returnvalue)))
        (Variables|Default|SetWords (.WordsandPhrases (Utilities|Struct|BreakDialogueStructure _returnvalue)))
        (Variables|Default|SetEquivalentWords (.LanguageEquivalents (Utilities|Struct|BreakDialogueStructure _returnvalue)))
        (Variables|Default|SetInLanguage (.InLanguage (Utilities|Struct|BreakDialogueStructure _returnvalue)))
        (Variables|Default|SetPlayerSpeaks (.PlayerSpeaks (Utilities|Struct|BreakDialogueStructure _returnvalue)))
        (Variables|Default|SetActivateQuest (.ActivateQuest (Utilities|Struct|BreakDialogueStructure _returnvalue)))
        (Variables|Default|SetGiveItem (.GiveItem (Utilities|Struct|BreakDialogueStructure _returnvalue)))
        (Utilities|FlowControl|Sequence
          (:then_0
            ;[1 1 1] Sets Dialogue
            (bind _output_get (Variables|Default|SetDialogue (.Dialogue (Utilities|Struct|BreakDialogueStructure _returnvalue))))
            (Default|SetText _dialoguecache _output_get (Utilities|String|ParseIntoArray (Variables|Default|GetWords) "\\") (Utilities|String|ParseIntoArray (Variables|Default|GetEquivalentWords) "\\") (Utilities|String|ParseIntoArray (Variables|Default|GetInLanguage) "\\"))
            (Variables|/Game/BluePrints/UI_Widgets/Pop-Ups/TextBox/Dialogue.Dialogue_C|SetSpanishDialogue _dialoguecache true))
          (:then_1
            ;[1 1 1] Changes Character text
            (if (Variables|Default|GetPlayerSpeaks)
              (Default|SetName (Variables|Default|GetDialogueCache) "Athel")
              (else
                (Default|SetName (Variables|Default|GetDialogueCache) (Utilities|Text|ToText(Name) (Variables|Default|GetCharacterName)))))))
        (else
          (CallFunction|EndDialogue))))
    (:RowNotFound
      (CallFunction|EndDialogue))))