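; Quest player state that links NPC interaction to the quest system and main game UI.
; On BeginPlay it creates and stores the example game main UI widget.
; Starting an NPC interaction reports the NPC to the QuestManager, completing the first dialog, then shows the talk tab and mouse cursor; stopping hides both.
; QuestManager accepted and completed events are bound but empty.
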(event QuestAccepted(QuestManager)
  (params (QuestSlot :type Integer) (Quest :type Quest%20Structure%20%28by%20ref%29)))

(event QuestCompleted(QuestManager)
  (params (Quest :type Quest%20Structure%20%28by%20ref%29) (CompletedSlot :type Integer)))

(event Custom|StartNPCInteract
  (params (NPCIN :type Actor%20Object%20Reference))
  (Class|QuestManager|ReachedNPC (Variables|Default|GetQuestManager) NPCIN true)
  (Widget|SetVisibility (Variables|/QuestEditor/Examples/Example_GameUI/WBP_ExampleGameMainUI.WBP_ExampleGameMainUI_C|GetTalkTab (Variables|Default|GetMainUI)) "Visible")
  (Variables|/Script/Engine.PlayerController|SetbShowMouseCursor (Game|GetPlayerController 0) true)
  (Variables|/Script/Engine.PlayerController|SetbEnableMouseOverEvents (Game|GetPlayerController 0) true))

(event Custom|StopNPCInteract
  (Widget|SetVisibility (Variables|/QuestEditor/Examples/Example_GameUI/WBP_ExampleGameMainUI.WBP_ExampleGameMainUI_C|GetTalkTab (Variables|Default|GetMainUI)) "Collapsed")
  (Variables|/Script/Engine.PlayerController|SetbShowMouseCursor (Game|GetPlayerController 0) false)
  (Variables|/Script/Engine.PlayerController|SetbEnableMouseOverEvents (Game|GetPlayerController 0) false))

(event EventBeginPlay
  (bind _returnvalue (UserInterface|CreateWidget "/QuestEditor/Examples/Example_GameUI/WBP_ExampleGameMainUI.WBP_ExampleGameMainUI_C"))
  (bind _output_get (Variables|Default|SetMainUI _returnvalue))
  (UserInterface|Viewport|AddtoViewport _output_get 0))

(fn ConstructionScript)