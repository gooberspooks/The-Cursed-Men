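; NPC dialogue Blueprint for quests that shows a dialogue widget and loads English or Spanish text.
; On BeginPlay it adds the widget to the viewport and shows the mouse cursor.
; SwitchDialogue reads a data table row by RowName, resets DialogueID, and fills Dialogue and Words in the language set by that row's InEnglish flag.
; AdvanceText is empty, and the event graph's SwitchDialogue call is unwired.
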(event Custom|AdvanceText)

(event EventBeginPlay
  (bind _returnvalue (Game|GetPlayerController 0))
  (bind _returnvalue_2 (UserInterface|CreateWidget "/Game/BluePrints/UI_Widgets/TextBox/Dialogue.Dialogue_C" _returnvalue))
  (UserInterface|Viewport|AddtoViewport _returnvalue_2 0)
  (Variables|/Script/Engine.PlayerController|SetbShowMouseCursor _returnvalue true))

(fn SwitchDialogue
  (bind _returnvalue (Utilities|GetDataTableRow "/Game/BluePrints/DataTables/Dialogue.Dialogue" (Variables|Default|GetRow%20Name))
    (:then
      (Variables|Default|SetDialogue%20ID 0)
      (bind _output_get (Variables|Default|SetInEnglish (.InEnglish (Utilities|Struct|BreakDialogueStructure _returnvalue))))
      (if _output_get
        (Variables|Default|SetDialogue (.EnglishEquivalent (Utilities|Struct|BreakDialogueStructure _returnvalue)))
        (Variables|Default|SetWords (.EnglishWordsandPhrases (Utilities|Struct|BreakDialogueStructure _returnvalue)))
        (else
          (Variables|Default|SetDialogue (.SpanishDialogue (Utilities|Struct|BreakDialogueStructure _returnvalue)))
          (Variables|Default|SetWords (.SpanishWordsandPhrases (Utilities|Struct|BreakDialogueStructure _returnvalue))))))
    (:RowNotFound
      (Development|PrintString "Error with reading data table"))))