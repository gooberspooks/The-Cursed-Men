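; Item component that adds its configured item to the player's inventory.
; AddItem casts the player character to BP_Athel and, if its Inventory is valid, passes it the ItemID row name and Quantity.
; The event graph holds only unconnected leftovers, including playtest slot-removal, data table lookup and owner-destroy nodes, so pickups do not destroy their owner here.
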(event EventBeginPlay
  ;[1 1 1] For playtesting add and remove item features. (Can delete when in actual use)
)

(event EventTick
  (params (DeltaSeconds :type Float%20%28single-precision%29))
  ;[1 1 1] For playtesting add and remove item features. (Can delete when in actual use)
)

(fn AddItem
  (bind _asbp_athel (Utilities|Casting|CastToBP_Athel (Game|GetPlayerCharacter 0)))
  (Utilities|IsValid (Variables|/Game/Character/Player/Athel/BP_Athel.BP_Athel_C|GetInventory _asbp_athel)
    (:Is%20Valid
      (Default|AddItem (Variables|/Game/Character/Player/Athel/BP_Athel.BP_Athel_C|GetInventory _asbp_athel) (.rowname (Variables|Default|GetItemID)) (Variables|Default|GetQuantity)))))