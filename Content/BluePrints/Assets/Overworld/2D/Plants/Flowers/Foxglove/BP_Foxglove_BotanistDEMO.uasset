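; Foxglove plant Blueprint, a demo variant tied to the Botanist NPC, that advances the Botanist's dialogue when harvested.
; HarvestPlant runs the parent harvest logic, then sets the Botanist's NPCDialogue ID and both its initial and current row numbers to fixed values.
; Construction defers to the parent, and the other default events are disabled stubs.
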(event EventBeginPlay
  (|CallParentFunction) ; This node is disabled and will not be called.\nDrag off pins to build functionality.
)

(event Collision|EventActorBeginOverlap
  (params (OtherActor :type Actor%20Object%20Reference))
  (|CallParentFunction OtherActor) ; This node is disabled and will not be called.\nDrag off pins to build functionality.
)

(event EventTick
  (params (DeltaSeconds :type Float%20%28single-precision%29))
  (|CallParentFunction DeltaSeconds) ; This node is disabled and will not be called.\nDrag off pins to build functionality.
)

(event EventHarvestPlant
  (bind _botanist (Variables|Default|GetBotanist))
  (bind _npcdialogue (Variables|/Game/Character/NPC/BP_NPCTemplate.BP_NPCTemplate_C|GetNPCDialogue _botanist))
  (|CallParentFunction)
  (Variables|/Game/BluePrints/Dialogue/NPCDialogue.NPCDialogue_C|SetDialogue%20ID _npcdialogue 4)
  (Variables|/Game/BluePrints/Dialogue/NPCDialogue.NPCDialogue_C|SetRow%20Number%20Initial _npcdialogue 28)
  (Variables|/Game/BluePrints/Dialogue/NPCDialogue.NPCDialogue_C|SetRow%20Number _npcdialogue 28))

(fn ConstructionScript
  (|CallParentFunction))