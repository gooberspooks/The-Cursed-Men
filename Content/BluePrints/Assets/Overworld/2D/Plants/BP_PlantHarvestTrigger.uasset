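; BP_PlantHarvestTrigger is an overlap trigger that lets the player character, BP_Athel, harvest a linked plant.
; Entering the trigger enables input on it and shows interact text on a referenced TextRenderActor, while leaving disables input and swaps the text.
; Pressing E calls HarvestPlant on the PlantPicked reference, then destroys the trigger.
; A node to destroy the text actor is present but unconnected.
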(event Custom|Activate%20Harvesting
  ;[1 1 1] Allows Harvesting of the plant
  (Input|EnableInput (Game|GetPlayerController 0))
  (Rendering|Components|TextRender|SetText (Variables|/Script/Engine.TextRenderActor|GetTextRender (Variables|Default|GetText%20Render%20Actor)) (Variables|Default|GetInteract%20Text)))

(event Custom|Deactivate%20Harvesting
  ;[1 1 1] Disables Harvesting of the plant
  (Input|DisableInput (Game|GetPlayerController 0))
  (Rendering|Components|TextRender|SetText (Variables|/Script/Engine.TextRenderActor|GetTextRender (Variables|Default|GetText%20Render%20Actor)) (Variables|Default|GetDisable%20Interact%20Text)))

(event Collision|EventActorBeginOverlap
  (params (OtherActor :type Actor%20Object%20Reference))
  ;[1 1 1] If Player is overlapping PlantHarvestTrigger, Allow Harvesting of the attached plant
  (if (== (Utilities|GetClass OtherActor) "/Game/Character/Player/Athel/BP_Athel.BP_Athel_C")
    (CallFunction|ActivateHarvesting)))

(event Collision|EventActorEndOverlap
  (params (OtherActor :type Actor%20Object%20Reference))
  ;[1 1 1] If Player stops overlapping PlantHarvestTrigger, Disallow Harvesting of the attached plant
  (if (== (Utilities|GetClass OtherActor) "/Game/Character/Player/Athel/BP_Athel.BP_Athel_C")
    (CallFunction|DeactivateHarvesting)))

(event Input|KeyboardEvents|E
  (params (Key :type Key%20Structure :default "None"))
  ;[1 1 1] When Player Presses [E] Harvest the Plant
  (:Pressed
    (Default|HarvestPlant (Variables|Default|GetPlant%20Picked))
    (Actor|DestroyActor)))

(fn ConstructionScript)