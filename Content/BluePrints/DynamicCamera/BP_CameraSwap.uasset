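; Trigger actor that blends the player's view to its own static camera while the player character is inside its overlap area.
; Begin overlap activates the camera and makes this actor the view target; end overlap blends back to the player character over the same swap time.
; A retriggerable delay then deactivates the idle camera, with a collision flag preventing shutdown if the player re-enters during the blend.
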(event Collision|EventActorEndOverlap
  (params (OtherActor :type Actor%20Object%20Reference))
  (if (== OtherActor (Game|GetPlayerCharacter 0))
    (Variables|Default|SetPlayerIsColliding false) ; Allowing camera deactivation
    (CallFunction|ReturnCamera) ; Swap to player camera
    (Utilities|FlowControl|RetriggerableDelay (Variables|Default|GetSwapTime)) ; Wait till transition completes
    (if (not (Variables|Default|GetPlayerIsColliding)) ; Preventing edge case glitch
      (Components|Activation|Deactivate (Variables|Default|GetCamera)) ; Turn off camera when not in use
    )))

(event Collision|EventActorBeginOverlap
  (params (OtherActor :type Actor%20Object%20Reference))
  (if (== OtherActor (Game|GetPlayerCharacter 0))
    (CallFunction|ControlCamera) ; Swap to static camera
    (Variables|Default|SetPlayerIsColliding true) ; Prevents deactivation of camera while inside
  ))

(fn ConstructionScript)

(fn ControlCamera
  (Components|Activation|Activate (Variables|Default|GetCamera) false)
  (Game|Player|SetViewTargetwithBlend (Game|GetPlayerController 0) self (Variables|Default|GetSwapTime) "VTBlend_Linear" 0.0 true))

(fn ReturnCamera
  (Game|Player|SetViewTargetwithBlend (Game|GetPlayerController 0) (Game|GetPlayerCharacter 0) (Variables|Default|GetSwapTime) "VTBlend_Linear" 0.0 true))